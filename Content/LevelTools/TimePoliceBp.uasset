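; Time police spawn point that, on the Active event, opens its child portal and sends a TimeCop out after a capture target.
; The portal opens with a sound and audible loop, then after a short delay plays an exit cue and spawns the cop.
; The cop's AI controller receives this actor as Home, plus Target and Closest as capture target and capturer.
; Construction places the camera from CamLocation, and BeginPlay disables the sphere's collision.
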(event `self.ReceiveBeginPlay`
  (`PrimitiveComponent.SetCollisionEnabled` (`self.Sphere`) "NoCollision"))

(event `Active`
  (bind _returnvalue (`self.K2_GetActorLocation`))
  (bind _asbp_portal (cast `/Game/VFX/BP_Portal` (`ChildActorComponent.ChildActor` (`self.BP_Portal`))))
  (`/Game/VFX/BP_Portal.Open` _asbp_portal)
  (`GameplayStatics.PlaySoundAtLocation` "/Game/Sounds/SoundsforSPotter/Portal/PortalOpen_Cue.PortalOpen_Cue" _returnvalue (struct) 1.0 1.0 0.0 null null null)
  (`AudioComponent.SetVolumeMultiplier` (`self.PortalLoop_Cue`) 1.0)
  (`KismetSystemLibrary.Delay` 1.0)
  (`GameplayStatics.PlaySoundAtLocation` "/Game/Sounds/SoundsforSPotter/Portal/PortalExit_Cue.PortalExit_Cue" _returnvalue (struct) 1.0 1.0 0.0 null null null)
  (bind _returnvalue_2 (`|SpawnActorFromClass` "/Game/AI/TImeCop/TimeCop.TimeCop_C" (`self.GetTransform`) "AlwaysSpawn" "OverrideRootScale" null null))
  (set `self.SpawnedCop` _returnvalue_2)
  (bind _ascop_controller (cast `/Game/AI/TImeCop/CopController` (`AIBlueprintHelperLibrary.GetAIController` _returnvalue_2)))
  (set `self.CopController` _ascop_controller)
  (set `/Game/AI/TImeCop/CopController.Home` self _ascop_controller)
  (set `/Game/AI/TImeCop/CopController.CaptureTarget` (`self.Target`) _ascop_controller)
  (set `/Game/AI/TImeCop/CopController.Capturer` (`self.Closest`) _ascop_controller))

(fn `UserConstructionScript`
  (`SceneComponent.K2_SetRelativeTransform` (`self.Camera`) (`self.CamLocation`) false false))