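; Environment controller that drives time of day, wind and a time-stop effect for the level.
; TimeUpdate lerps fog color, sun rotation and intensity, sphere scale and the MP_Global time parameter from one alpha.
; ChangeWindDirection cycles an array, blending the vector by timeline into MP_Global and the wind source's speed and yaw.
; TimeStop swaps in a frozen sky, fades in a post-process material, zeroes material wind, disables actor physics and notifies Bards and Waterwheel.
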(event `TimeStop`
  ;[1 1 1] Time Stop
  (`PrimitiveComponent.SetMaterial` (`self.SM_Skysphere`) 0 "/Game/Materials/M_Sky_Frozen.M_Sky_Frozen")
  (`|ExecutionSequence`
    (:`then_0`
      (`KismetMaterialLibrary.SetVectorParameterValue` "/Game/AI/EnvironmentBPs/MP_Global.MP_Global" "Wind Direction" (`KismetMathLibrary.Conv_ColorToLinearColor` (make `Color` 0))) ; Stop Wind
    )
    (:`then_1`
      (bind _returnvalue (`KismetMaterialLibrary.CreateDynamicMaterialInstance` "/Game/Materials/PPM_TimeFrozen.PPM_TimeFrozen"))
      (bind _output_get (set `self.PPM_TimeFrozen` _returnvalue))
      (setmembers `PostProcessSettings` :`StructRef` (`PostProcessComponent.Settings` (`self.PostProcess`)) :`WeightedBlendables` (make `WeightedBlendables` (`|MakeArray` (make `WeightedBlendable` 1.0 _output_get))))
      (bind (_direction _fadein) (`Timeline|Timeline_0` :!via `PlayFromStart`)
        (:`Update`
          (`MaterialInstanceDynamic.SetScalarParameterValue` (`self.PPM_TimeFrozen`) "Strength" _fadein))))
    (:`then_2`
      (`KismetMaterialLibrary.SetVectorParameterValue` "/Game/AI/EnvironmentBPs/MP_Global.MP_Global" "Wind Direction" (`KismetMathLibrary.LinearColor_Black`)))
    (:`then_3`
      (for _array_element (`self.PhysicsActors`)
        (`PrimitiveComponent.SetSimulatePhysics` (`StaticMeshActor.StaticMeshComponent` _array_element) false)))
    (:`then_4`
      (for _array_element_2 (`self.Bards`)
        (`/Game/AI/Bard.TimeStopped` _array_element_2)))
    (:`then_5`
      (`/Game/AI/EnvironmentBPs/BP_Waterwheel.Time Stopped` (`self.Waterwheel`)))))

(event `self.ReceiveBeginPlay`
  (bind _skymaterial (`self.SkyMaterial`))
  (bind _component (`WindDirectionalSource.Component` (`self.Wind Source`)))
  ;[1 1 1] Setup
  (bind _returnvalue (`KismetMaterialLibrary.CreateDynamicMaterialInstance` "/Game/Materials/M_Sky.M_Sky"))
  (bind _output_get (set `self.SkyMaterial` _returnvalue))
  (`PrimitiveComponent.SetMaterial` (`self.SM_Skysphere`) 0 _output_get)
  (`MaterialInstanceDynamic.SetVectorParameterValue` _skymaterial "StartColor" (`self.SkyStartColor`))
  (`MaterialInstanceDynamic.SetVectorParameterValue` _skymaterial "EndColor" (`self.SkyEndColor`))
  (`WindDirectionalSourceComponent.SetStrength` _component 500.0)
  (`WindDirectionalSourceComponent.SetSpeed` _component 150.0)
  (`SceneComponent.K2_SetWorldRotation` :`self` _component)
  (`|ExecutionSequence`
    (:`then_0`
      (set `self.Current Wind Array Value` -1) ; keep this stuff
    )))

(event `Change Wind Direction`
  (bind _returnvalue (+ (`self.Current Wind Array Value`) 1))
  (bind _component (`WindDirectionalSource.Component` (`self.Wind Source`)))
  ;[1 1 1] Wind Direction
  ;;[1 1 1] Find the target wind direction
  (if (> _returnvalue (- (`KismetArrayLibrary.Array_Length` (`self.Wind Directions Array`)) 1))
    (set `self.Current Wind Array Value` 0) ; Reset the array
    (else
      (set `self.Current Wind Array Value` _returnvalue) ; Go to the next value in the wind directions array
    ))
  (set `self.Target Wind Direction` (`|GetArrayItem` (`self.Wind Directions Array`) (`self.Current Wind Array Value`)))
  ;;[1 1 1] Lerp old direction to new
  (bind (_direction _newtrack_0) (`Timeline|WindLerp` :!via `PlayFromStart`)
    (:`Update`
      (bind _returnvalue_2 (`KismetMathLibrary.VLerp` (`self.Current Wind Direction`) (`self.Target Wind Direction`) _newtrack_0))
      (`KismetMaterialLibrary.SetVectorParameterValue` "/Game/AI/EnvironmentBPs/MP_Global.MP_Global" "Wind Direction" (`KismetMathLibrary.Conv_VectorToLinearColor` _returnvalue_2))
      (bind (_returnvalue_x _returnvalue_y) (`KismetMathLibrary.BreakVector` (+ _returnvalue_2 (0.0 0.0 0.0))))
      (`WindDirectionalSourceComponent.SetSpeed` _component (`KismetMathLibrary.Lerp` 0.0 150.0 (+ (`KismetMathLibrary.Abs` _returnvalue_x) (`KismetMathLibrary.Abs` _returnvalue_y))))
      (`SceneComponent.K2_SetWorldRotation` _component (`KismetMathLibrary.MakeRotator` 0.0 0.0 (`KismetMathLibrary.DegAtan2` _returnvalue_y _returnvalue_x)) false false))
    (:`Finished`
      (set `self.Current Wind Direction` (`self.Target Wind Direction`)))))

(event `TimeUpdate`
  (params (Lerp :type "Float (double-precision)"))
  ;[1 1 1] Time of Day
  (`KismetSystemLibrary.PrintString` (`KismetStringLibrary.Conv_DoubleToString` Lerp))
  (`ExponentialHeightFogComponent.SetFogInscatteringColor` (`self.ExponentialHeightFog`) (`KismetMathLibrary.LinearColorLerp` (`self.Fog Start Color`) (`self.Fog End Color`) Lerp)) ; Update the color of the exponential hight fog
  (`SceneComponent.K2_SetWorldRotation` (`self.Sun Rotation Axis`) (`KismetMathLibrary.RLerp` (struct) (struct :`Roll` -130.0) Lerp) true false) ; Update Sun Pos
  (`LightComponent.SetIntensity` (`self.Sunlight`) (`KismetMathLibrary.Lerp` 3.141593 1.5 Lerp)) ; Update sunlight brightness
  (`KismetMaterialLibrary.SetScalarParameterValue` "/Game/AI/EnvironmentBPs/MP_Global.MP_Global" "Time of Day" Lerp) ; Update material param for clouds, sky color, clouds outline, etc...
  (`SceneComponent.SetWorldScale3D` (`self.Sphere`) (`KismetMathLibrary.Conv_DoubleToVector` (`KismetMathLibrary.Lerp` 60.0 120.0 Lerp))))

(fn `UserConstructionScript`)