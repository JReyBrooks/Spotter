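; In-world computer screen for the main menu, driving a MainMenuUI widget through a virtual cursor.
; The first left click activates the screen and hides the system cursor; later clicks, and touch releases, call the widget's Click.
; While active, Tick traces from the mouse, moves WidgetInteraction to the hit and offsets the UI cursor, snapping the mouse back when off-screen.
; BeginPlay also destroys the DefaultPawn.
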(event `self.ReceiveTick`
  (params (DeltaSeconds :type "Float (single-precision)"))
  (bind _returnvalue (`GameplayStatics.GetPlayerController` 0))
  (bind _returnvalue_2 (`GameplayStatics.GetPlayerController` 0))
  (bind _widgetinteraction (`self.WidgetInteraction`))
  (bind (_mousepos_x _mousepos_y) (`KismetMathLibrary.BreakVector` (`self.MousePos`)))
  (bind (_worldlocation _worlddirection) (`PlayerController.DeprojectMousePositionToWorld` _returnvalue))
  (bind (_returnvalue_x _returnvalue_y) (`KismetMathLibrary.BreakVector2D` (`WidgetInteractionComponent.Get2DHitLocation` _widgetinteraction)))
  (bind (_locationx _locationy) (`PlayerController.GetMousePosition` _returnvalue_2))
  (if (`self.ComputerScreen`)
    (bind _outhit (`KismetSystemLibrary.LineTraceSingleForObjects` _worldlocation (+ _worldlocation (* _worlddirection 150.0)) (`self.UIelements`) true (`|MakeArray` (`Controller.K2_GetPawn` _returnvalue) :!type "Actor Object Reference")))
    (if (`GameplayStatics.BreakHitResult` _outhit)
      (bind _output_get (set `self.MousePos` (`KismetMathLibrary.MakeVector` _locationx _locationy)))
      (`SceneComponent.K2_SetWorldLocation` _widgetinteraction (`KismetMathLibrary.MakeVector` (.x (`.Location` (`GameplayStatics.BreakHitResult` _outhit))) (+ (.y (`.Location` (`GameplayStatics.BreakHitResult` _outhit))) -1.0) (.z (`.Location` (`GameplayStatics.BreakHitResult` _outhit)))) true false)
      (bind _asmain_menu_ui (cast `/Game/Maps/MainMenuStuff/MainMenuUI` (`WidgetComponent.GetWidget` (`self.Widget`))))
      (set `/Game/Maps/MainMenuStuff/MainMenuUI.Translation` (`KismetMathLibrary.MakeVector2D` (+ _returnvalue_x -975.0) (+ _returnvalue_y -550.0)) _asmain_menu_ui)
      (else
        (`PlayerController.SetMouseLocation` _returnvalue_2 (`KismetMathLibrary.FTrunc` _mousepos_x) (`KismetMathLibrary.FTrunc` _mousepos_y))))))

(event `self.ReceiveBeginPlay`
  (bind _returnvalue (`GameplayStatics.GetActorOfClass` "/Script/Engine.DefaultPawn"))
  (`self.K2_DestroyActor` _returnvalue))

(event `InputTouch`
  (params (Location :type "Vector Structure") (FingerIndex :type "ETouchIndex Enum"))
  (:`Released`
    (bind _asmain_menu_ui (cast `/Game/Maps/MainMenuStuff/MainMenuUI` (`WidgetComponent.GetWidget` (`self.Widget`)) :!label _label))
    (`/Game/Maps/MainMenuStuff/MainMenuUI.Click` _asmain_menu_ui)))

(event `Key|LeftMouseButton`
  (params (Key :type "Key Structure"))
  (bind _returnvalue (`GameplayStatics.GetPlayerController` 0))
  (:`Pressed`
    (`|ExecutionSequence`
      (:`then_0`
        (`/Engine/EditorBlueprintResources/StandardMacros.Gate` true :!label _label_2
          (:`Exit`
            (goto _label))))
      (:`then_1`
        (`/Engine/EditorBlueprintResources/StandardMacros.DoOnce` false
          (:`Completed`
            (set `self.ComputerScreen` true)
            (set `PlayerController.bShowMouseCursor` false _returnvalue)
            (`WidgetBlueprintLibrary.SetInputMode_GameOnly` _returnvalue)
            (`PlayerController.SetMouseLocation` _returnvalue 450 450)
            (goto _label_2 :!via `Open`)))))))

(fn `UserConstructionScript`)